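; Inventory actor component that stores an owner's items in an Items array without duplicates.
; It offers functions to check, remove and add items, with ReplaceItem adding the new item only if removing the old one succeeds.
; AddItem returns true when AddUnique yields -1, meaning the item was already present, and ReplaceItem passes that result through.
; BeginPlay adds the cube item asset twice, apparently as a test.
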(event EventBeginPlay
  (CallFunction|AddItem "/Game/Blueprint/Inventory/Items/DA_Item_Cube.DA_Item_Cube")
  (CallFunction|AddItem "/Game/Blueprint/Inventory/Items/DA_Item_Cube.DA_Item_Cube"))

(fn HasItem
  (params (Item :type BP%20DA%20Item%20Object%20Reference))
  (return (Utilities|Array|ContainsItem (Variables|Default|GetItems) Item)))

(fn RemoveItem
  (params (Item :type BP%20DA%20Item%20Object%20Reference))
  (bind _returnvalue (Utilities|Array|RemoveItem (Variables|Default|GetItems) Item))
  (return _returnvalue))

(fn AddItem
  (params (Item :type BP%20DA%20Item%20Object%20Reference))
  (bind _returnvalue (Utilities|Array|AddUnique (Variables|Default|GetItems) Item))
  (return (== _returnvalue -1)))

(fn ReplaceItem
  (params (OldItem :type BP%20DA%20Item%20Object%20Reference) (NewItem :type BP%20DA%20Item%20Object%20Reference))
  (bind _returnvalue (CallFunction|RemoveItem OldItem))
  (if _returnvalue
    (bind _returnvalue_2 (CallFunction|AddItem NewItem))
    (return _returnvalue_2)
    (else
      (return false))))