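; Inventory item preview actor that films an item's mesh with a scene capture limited to its own components, for render target display.
; LaunchCapture applies the item's mesh and scale and enables per-frame capture and rotation; StopCapture clears the mesh and disables both.
; While active, IA_Look input yaws a socket component and pitches the mesh, scaled by speed and delta time.
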(event Custom|LaunchCapture
  (params (Item :type BP%20DA%20Item%20Object%20Reference))
  (Components|StaticMesh|SetStaticMesh (Variables|Default|GetStaticMesh) (Variables|/Game/Blueprint/Inventory/BP_DA_Item.BP_DA_Item_C|GetMesh Item))
  (Variables|/Script/Engine.SceneCaptureComponent|SetbCaptureEveryFrame (Variables|Default|GetSceneCaptureComponent2D) true)
  (Variables|Default|SetMovement true)
  (Transformation|SetRelativeScale3D (Variables|Default|GetStaticMesh) (Variables|/Game/Blueprint/Inventory/BP_DA_Item.BP_DA_Item_C|GetMeshScale Item)))

(event Custom|StopCapture
  (Components|StaticMesh|SetStaticMesh (Variables|Default|GetStaticMesh) 0)
  (Variables|/Script/Engine.SceneCaptureComponent|SetbCaptureEveryFrame (Variables|Default|GetSceneCaptureComponent2D) false)
  (Variables|Default|SetMovement false))

(event Input|EnhancedActionEvents|EnhancedInputActionIA_Look
  (params (ActionValue :type Vector%202D%20Structure) (ElapsedSeconds :type Float%20%28double-precision%29) (TriggeredSeconds :type Float%20%28double-precision%29) (InputAction :type Input%20Action%20Object%20Reference :default "/Game/Input/Actions/IA_Look.IA_Look"))
  (bind _returnvalue (Utilities|Time|GetWorldDeltaSeconds))
  (if (Variables|Default|GetMovement)
    (Transformation|AddLocalRotation (Variables|Default|GetYawSocket) (Math|Rotator|MakeRotator 0.0 0.0 (CallFunction|KL-x (* (.x ActionValue) (Variables|Default|GetYawSpeed) _returnvalue))) false false)
    (Transformation|AddLocalRotation (Variables|Default|GetStaticMesh) (Math|Rotator|MakeRotator 0.0 (* (.y ActionValue) (Variables|Default|GetPitchSpeed) _returnvalue) 0.0) false false)))

(event EventBeginPlay
  (Rendering|SceneCapture|ShowOnlyActorComponents (Variables|Default|GetSceneCaptureComponent2D) self false))

(fn ConstructionScript)