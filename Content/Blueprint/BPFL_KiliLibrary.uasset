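; Kili's general-purpose Blueprint function library of math, random and array helpers, with a KLHelp graph of unexecuted usage examples.
; Weighted random pickers walk cumulative weights using a random stream to return an index.
; Other helpers cover dot-product facing checks, line trace endpoints, polar-to-Cartesian conversion, timer updates by reference and one-minus.
; It also bubble-sorts floats in descending order and builds random pseudonyms from two word lists.
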(fn ==KLHelp==)

(fn KLWeightedRandomInt
  (params (Stream :type Random%20Stream%20Structure) (Weights :type Array%20of%20Integers))
  (for _array_element Weights
    (LocalVariables|SetSumOfWeights (+ (LocalVariables|GetSumOfWeights) _array_element)))
  (LocalVariables|SetRandomInt (Class|KismetMathLibrary|RandomIntegerfromStream Stream (LocalVariables|GetSumOfWeights)))
  (LocalVariables|SetTempRarity 0)
  (bind (_array_element_2 _array_index) (Utilities|Array|ForEachLoopwithBreak Weights :!label _label)
    (:LoopBody
      (if (and (>= (LocalVariables|GetRandomInt) (LocalVariables|GetTempRarity)) (< (LocalVariables|GetRandomInt) (+ (LocalVariables|GetTempRarity) _array_element_2)))
        (LocalVariables|SetFoundItem _array_index)
        (goto _label Break)
        (else
          (LocalVariables|SetTempRarity (+ _array_element_2 (LocalVariables|GetTempRarity))))))
    (:Completed
      (return (LocalVariables|GetFoundItem)))))

(fn KLWeightedRandomFloat
  (params (Stream :type Random%20Stream%20Structure) (Weights :type Array%20of%20Floats%20%28double-precision%29))
  (for _array_element Weights
    (LocalVariables|SetSumOfWeights (+ (LocalVariables|GetSumOfWeights) _array_element)))
  (LocalVariables|SetRandomFloat (Math|Random|RandomFloatinRangefromStream Stream 0.0 (LocalVariables|GetSumOfWeights)))
  (bind (_array_element_2 _array_index) (Utilities|Array|ForEachLoopwithBreak Weights :!label _label)
    (:LoopBody
      (if (and (>= (LocalVariables|GetRandomFloat) (LocalVariables|GetTempRarity)) (< (LocalVariables|GetRandomFloat) (+ (LocalVariables|GetTempRarity) _array_element_2)))
        (LocalVariables|SetFoundItem _array_index)
        (goto _label Break)
        (else
          (LocalVariables|SetTempRarity (+ _array_element_2 (LocalVariables|GetTempRarity))))))
    (:Completed
      (return (LocalVariables|GetFoundItem)))))

(fn KLRandomStream
  (return (Math|Random|MakeRandomStream (Math|Random|RandomInteger 2147483647))))

(fn KLIsBinFrontOfA
  (params (APos :type Vector) (AForward :type Vector) (BPos :type Vector) (Acceptance :type Float%20%28double-precision%29))
  (bind _output_get (LocalVariables|SetTempDot (Math|Vector|DotProduct (Math|Vector|Normalize (- BPos APos)) AForward)))
  (return (>= _output_get Acceptance) _output_get))

(fn KLConvertTrigCoordtoOrtho
  (params (Angle :type Float%20%28double-precision%29) (Radius :type Float%20%28double-precision%29) (RadAngle :type Boolean))
  (bind _returnvalue (Math|Trig|DegreesToRadians Angle))
  (bind _returnvalue_2 (Math|Float|SelectFloat Angle _returnvalue RadAngle))
  (return (Math|Vector2D|MakeVector2D (* (Math|Trig|Cos(Radians) _returnvalue_2) Radius) (* Radius (Math|Trig|Sin(Radians) _returnvalue_2)))))

(fn KLGetLinetraceGoal
  (params (StartPos :type Vector) (Direction :type Vector) (StartOffset :type Float%20%28double-precision%29) (EndOffset :type Float%20%28double-precision%29))
  (return (+ StartPos (* Direction StartOffset)) (+ StartPos (* Direction EndOffset))))

(fn KLUpdateTimer
  (params (Timer :type Float%20%28double-precision%29%20%28by%20ref%29) (DeltaTime :type Float%20%28double-precision%29) (Decrement :type Boolean))
  (|SetBy-RefVar Timer (Math|Float|SelectFloat (- Timer DeltaTime) (+ Timer DeltaTime) Decrement)))

(fn KLBubbleSortFloat
  (params (Array :type Array%20of%20Floats%20%28double-precision%29))
  (bind _output_get (LocalVariables|SetTempArray Array))
  (for (_array_element _array_index) _output_get :!label _label
    ;[0.03857 0.4115 0.284 0.5] Comparator
    (if (< _array_element (Utilities|Array|Get(acopy) _output_get (+ _array_index 1)))
      (Utilities|Array|Swap _output_get _array_index (+ _array_index 1))
      (LocalVariables|SetChangesMade true)))
  (if (LocalVariables|GetChangesMade)
    (LocalVariables|SetChangesMade false)
    (goto _label)
    (else
      (return (LocalVariables|GetTempArray)))))

(fn KL1-x
  (params (x :type Float%20%28double-precision%29))
  (return (- 1.0 x)))

(fn KLRandomPseudo
  (return (Utilities|String|Append (Utilities|Array|Get(acopy) (LocalVariables|Get1stWord) (Math|Random|RandomInteger (Utilities|Array|Length (LocalVariables|Get1stWord)))) (Utilities|Array|Get(acopy) (LocalVariables|Get2ndWord) (Math|Random|RandomInteger (Utilities|Array|Length (LocalVariables|Get2ndWord)))))))