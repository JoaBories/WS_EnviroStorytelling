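; BP_DoorChild_ChurchR is a child door Blueprint for what appears to be the right church door, with a mask piece mesh that depends on the player's inventory.
; MaskR is hidden at BeginPlay.
; On Interacted, MaskR becomes visible only if the player's BP_AC_Inventory holds DA_Item_Mask1stHalf, then the parent's interaction logic runs.
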(event EventBeginPlay
  (|CallParentFunction)
  (Rendering|SetVisibility (Variables|Default|GetMask_R) false false))

(event Collision|EventActorBeginOverlap
  (params (OtherActor :type Actor%20Object%20Reference))
  (|CallParentFunction OtherActor) ; This node is disabled and will not be called.\nDrag off pins to build functionality.
)

(event EventTick
  (params (DeltaSeconds :type Float%20%28single-precision%29))
  (|CallParentFunction DeltaSeconds) ; This node is disabled and will not be called.\nDrag off pins to build functionality.
)

(event EventInteracted
  (Rendering|SetVisibility (Variables|Default|GetMask_R) (Default|HasItem (Actor|GetComponentbyClass (Game|Player|GetPlayerPawn 0) "/Game/Blueprint/Inventory/BP_AC_Inventory.BP_AC_Inventory_C") "/Game/Blueprint/Inventory/Items/DA_Item_Mask1stHalf.DA_Item_Mask1stHalf") false)
  (|CallParentFunction))

(fn ConstructionScript
  (|CallParentFunction))