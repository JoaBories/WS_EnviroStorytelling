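; Interactable pedestal whose artefact triggers the game's ending sequence.
; Shows an outline overlay on the artefact until used, then disables player input and keeps steering the first-person camera toward it on Tick.
; A timeline moves the cut mesh with a knife sound, then the creature death plays sound and camera shake, restores input, moves the "Fog"-tagged actor along Y and opens the end menu.
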(event Custom|CutSequence
  (Rendering|SetVisibility (Variables|Default|GetCut) true false)
  (bind _t (Timeline|CutMovement Play)
    (:Update
      (Transformation|SetRelativeLocation (Variables|Default|GetCut) (Math|Vector|Lerp(Vector) (Variables|/Script/Engine.SceneComponent|GetRelativeLocation (Variables|Default|GetCutStart)) (Variables|/Script/Engine.SceneComponent|GetRelativeLocation (Variables|Default|GetCutEnd)) _t) false false))
    (:Finished
      (Audio|PlaySound2D (Variables|/Game/Blueprint/DataAssets/BPDA_ArtifactFeedbacks.BPDA_ArtifactFeedbacks_C|GetSoundKnife (Variables|Default|GetFeedbacks)) 1.0 1.0 0.0 0 0)
      (Utilities|FlowControl|Delay 1.0)
      (CallFunction|CreatureDeath))))

(event Custom|CreatureDeath
  (bind _fog (Variables|Default|GetFog))
  (bind _returnvalue (Transformation|GetActorLocation _fog))
  (Audio|PlaySound2D (Variables|/Game/Blueprint/DataAssets/BPDA_ArtifactFeedbacks.BPDA_ArtifactFeedbacks_C|GetSoundCreature (Variables|Default|GetFeedbacks)) 1.0 1.0 0.0 0 0)
  (CameraShakes|StartCameraShake (Game|GetPlayerCameraManager 0) "/Game/Blueprint/DataAssets/CS_CreatureDeath.CS_CreatureDeath_C" 1.0 "CameraLocal" "0, 0, 0")
  (Input|EnableInput (Variables|Default|GetChara) (Game|GetPlayerController 0))
  (bind _ylocation (Timeline|FogMovement Play)
    (:Update
      (Transformation|SetActorLocation _fog (Math|Vector|MakeVector (.x _returnvalue) _ylocation (.z _returnvalue)) false false))
    (:Finished
      (Utilities|FlowControl|Delay 1.0)
      (Game|OpenLevel(byObjectReference) "/Game/Level/L_EndMenu.L_EndMenu"))))

(event Collision|EventActorBeginOverlap
  (params (OtherActor :type Actor%20Object%20Reference)))

(event EventShowWidget
  (if (not (Variables|Default|GetActivated))
    (Rendering|Material|SetOverlayMaterial (Variables|Default|GetArtefact) "/Game/Blueprint/GPE/M_Outline.M_Outline" :!class /Script/Engine.MeshComponent)))

(event EventHideWidget
  (Rendering|Material|SetOverlayMaterial (Variables|Default|GetArtefact) 0 :!class /Script/Engine.MeshComponent))

(event EventInteracted
  (Variables|Default|SetActivated true)
  (Input|DisableInput (Variables|Default|GetChara) (Game|GetPlayerController 0))
  (CallFunction|CutSequence))

(event EventTick
  (params (DeltaSeconds :type Float%20%28single-precision%29))
  (bind _chara (Variables|Default|GetChara))
  (bind _firstpersoncamera (Variables|/Game/Blueprint/Player/BP_FirstPersonCharacter.BP_FirstPersonCharacter_C|GetFirstPersonCamera _chara))
  (if (Variables|Default|GetActivated)
    (Transformation|SetWorldRotation _firstpersoncamera (Math|Interpolation|RInterpTo (Transformation|GetWorldRotation _firstpersoncamera) (Math|Rotator|FindLookatRotation (Transformation|GetWorldLocation _firstpersoncamera) (Transformation|GetWorldLocation (Variables|Default|GetArtefact))) DeltaSeconds 5.0) false false)))

(event EventBeginPlay
  (Variables|Default|SetChara (.AsBP%20First%20Person%20Character (Utilities|Casting|CastToBP_FirstPersonCharacter (Game|GetPlayerCharacter 0))))
  (bind _outactors (Actor|GetAllActorswithTag "Fog"))
  (Variables|Default|SetFog (Utilities|Array|Get(acopy) _outactors)))

(fn ConstructionScript)