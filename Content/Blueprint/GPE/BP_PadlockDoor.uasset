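; BP_PadlockDoor is an interactable door held shut by a padlock that requires a code.
; Interacting while locked opens a WBP_Padlock widget, whose code validation event calls RemoveLock.
; RemoveLock marks the door unlocked and drops the padlock with physics, so the next interaction calls OpenDoor.
; Show/HideWidget events toggle an outline overlay material on the padlock, or on the door once unlocked.
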(event Custom|RemoveLock
  (bind _padlock (Variables|Default|GetPadlock))
  (Variables|Default|SetUnlocked true)
  (Collision|SetCollisionEnabled _padlock "PhysicsOnly")
  (Physics|SetSimulatePhysics _padlock true)
  (Rendering|Material|SetOverlayMaterial _padlock 0 :!class /Script/Engine.MeshComponent))

(event EventBeginPlay
  (|CallParentFunction) ; This node is disabled and will not be called.\nDrag off pins to build functionality.
)

(event Collision|EventActorBeginOverlap
  (params (OtherActor :type Actor%20Object%20Reference))
  (|CallParentFunction OtherActor) ; This node is disabled and will not be called.\nDrag off pins to build functionality.
)

(event EventTick
  (params (DeltaSeconds :type Float%20%28single-precision%29))
  (|CallParentFunction DeltaSeconds) ; This node is disabled and will not be called.\nDrag off pins to build functionality.
)

(event EventShowWidget
  (Rendering|Material|SetOverlayMaterial (select (Variables|Default|GetUnlocked) (Variables|Default|GetDoor) (Variables|Default|GetPadlock)) "/Game/Blueprint/GPE/M_Outline.M_Outline" :!class /Script/Engine.MeshComponent))

(event EventHideWidget
  (if (not (Variables|Default|GetisOpened))
    (Rendering|Material|SetOverlayMaterial (select (Variables|Default|GetUnlocked) (Variables|Default|GetDoor) (Variables|Default|GetPadlock)) 0 :!class /Script/Engine.MeshComponent)))

(event EventInteracted
  (if (Variables|Default|GetUnlocked)
    (if (not (Variables|Default|GetisOpened))
      (CallFunction|OpenDoor))
    (else
      (bind _returnvalue (UserInterface|CreateWidget "/Game/Blueprint/Uis/WBP_Padlock.WBP_Padlock_C"))
      (UserInterface|Viewport|AddtoViewport _returnvalue 10)
      (Class|CommonActivatableWidget|ActivateWidget _returnvalue)
      (EventDispatchers|BindEventtoValidateCode _returnvalue (delegate Custom|RemoveLock)))))

(fn ConstructionScript
  (|CallParentFunction))