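; BP_CrouchTriggerBox is a trigger volume that shows a crouch prompt to the player.
; When the player character overlaps the Box, it creates a WBP_CrouchPrompt widget and adds it to the viewport, and leaving the Box kills and clears it.
; Pressing IA_Crouch while the prompt exists kills it and destroys the actor, so a completed prompt does not reappear.
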(event OnComponentBeginOverlap(Box)
  (params (OverlappedComponent :type Primitive%20Component%20Object%20Reference) (OtherActor :type Actor%20Object%20Reference) (OtherComp :type Primitive%20Component%20Object%20Reference) (OtherBodyIndex :type Integer) (bFromSweep :type Boolean) (SweepResult :type Hit%20Result%20Structure%20%28by%20ref%29))
  (if (== OtherActor (Game|GetPlayerCharacter 0))
    (Variables|Default|GetPrompt
      (:then)
      (:else
        (bind _returnvalue (UserInterface|CreateWidget "/Game/Blueprint/Uis/WBP_CrouchPrompt.WBP_CrouchPrompt_C"))
        (bind _output_get (Variables|Default|SetPrompt _returnvalue))
        (UserInterface|Viewport|AddtoViewport _output_get 0)))))

(event OnComponentEndOverlap(Box)
  (params (OverlappedComponent :type Primitive%20Component%20Object%20Reference) (OtherActor :type Actor%20Object%20Reference) (OtherComp :type Primitive%20Component%20Object%20Reference) (OtherBodyIndex :type Integer))
  (if (== OtherActor (Game|GetPlayerCharacter 0))
    (bind _prompt (Variables|Default|GetPrompt)
      (:then
        (Default|Kill _prompt)
        (Variables|Default|SetPrompt 0))
      (:else))))

(event Input|EnhancedActionEvents|EnhancedInputActionIA_Crouch
  (params (ActionValue :type Boolean) (ElapsedSeconds :type Float%20%28double-precision%29) (TriggeredSeconds :type Float%20%28double-precision%29) (InputAction :type Input%20Action%20Object%20Reference :default "/Game/Input/Actions/IA_Crouch.IA_Crouch"))
  (bind _prompt (Variables|Default|GetPrompt)
    (:then
      (Default|Kill _prompt)
      (Actor|DestroyActor))
    (:else)))

(fn ConstructionScript)