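; BP_Door is an interactable door that opens once, optionally requiring every listed item to be in the player's BP_AC_Inventory component.
; Showing the widget applies an outline overlay material while the door is closed, and hiding it clears the overlay.
; Interacting checks the items, then plays a sound and a timeline that swings the mesh on yaw, with invertible direction.
; A separate OpenDoor event opens it without any checks.
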(event Custom|Open%20Door
  (Variables|Default|SetisOpened true)
  (CallFunction|HideWidget)
  (Audio|PlaySoundatLocation (Variables|Default|GetOpenSound) (Transformation|GetActorLocation) "0, 0, 0" 1.0 1.0 0.0 0 0 0 0)
  (bind _door_rotation (Timeline|OpenDoor PlayFromStart)
    (:Update
      (Transformation|SetRelativeRotation (Variables|Default|GetDoor) (Math|Rotator|MakeRotator 0.0 0.0 (* _door_rotation (Math|Float|SelectFloat -1.0 1.0 (Variables|Default|GetinvertOpenRotation)))) false false))))

(event EventBeginPlay)

(event Collision|EventActorBeginOverlap
  (params (OtherActor :type Actor%20Object%20Reference)))

(event EventTick
  (params (DeltaSeconds :type Float%20%28single-precision%29)))

(event EventShowWidget
  (if (not (Variables|Default|GetisOpened))
    (Rendering|Material|SetOverlayMaterial (Variables|Default|GetDoor) "/Game/Blueprint/GPE/M_Outline.M_Outline" :!class /Script/Engine.MeshComponent)))

(event EventHideWidget
  (Rendering|Material|SetOverlayMaterial (Variables|Default|GetDoor) 0 :!class /Script/Engine.MeshComponent))

(event EventInteracted
  (if (not (Variables|Default|GetisOpened))
    (if (Utilities|Array|IsNotEmpty (Variables|Default|GetNeededItem))
      (Variables|Default|SethasEveryItems true)
      (for _array_element (Variables|Default|GetNeededItem)
        (if (not (Default|HasItem (Actor|GetComponentbyClass (Game|Player|GetPlayerPawn 0) "/Game/Blueprint/Inventory/BP_AC_Inventory.BP_AC_Inventory_C") _array_element))
          (Variables|Default|SethasEveryItems false)))
      (if (Variables|Default|GethasEveryItems)
        (Variables|Default|SetisOpened true :!label _label)
        (CallFunction|HideWidget)
        (Audio|PlaySoundatLocation (Variables|Default|GetOpenSound) (Transformation|GetActorLocation) "0, 0, 0" 1.0 1.0 0.0 0 0 0 0)
        (bind _door_rotation (Timeline|OpenDoor PlayFromStart)
          (:Update
            (Transformation|SetRelativeRotation (Variables|Default|GetDoor) (Math|Rotator|MakeRotator 0.0 0.0 (* _door_rotation (Math|Float|SelectFloat -1.0 1.0 (Variables|Default|GetinvertOpenRotation)))) false false))))
      (else
        (goto _label)))))

(fn ConstructionScript)

(fn GetPrompt
  (return "Open"))