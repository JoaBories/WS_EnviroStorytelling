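; BP_PhotoToTake is an interactable photo pickup that the first-person player collects by interacting with it.
; On interaction it hides itself, triggers the player character's TakePhoto, waits briefly, then adds its Item to the player's inventory component.
; It starts an optional collection dialogue on the player's HUD if one is set, then destroys itself.
; The construction script applies the PhotoFrame mesh to its static mesh.
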(event EventBeginPlay)

(event Collision|EventActorBeginOverlap
  (params (OtherActor :type Actor%20Object%20Reference)))

(event EventTick
  (params (DeltaSeconds :type Float%20%28single-precision%29)))

(event EventInteracted
  (bind _returnvalue (Game|GetPlayerCharacter 0))
  (bind _dialoguewhencollecting (Variables|Default|GetDialogueWhenCollecting))
  (bind _asbp_first_person_character (Utilities|Casting|CastToBP_FirstPersonCharacter _returnvalue))
  (Rendering|SetVisibility (Variables|Default|GetDefaultSceneRoot) false true)
  (Default|TakePhoto _asbp_first_person_character)
  (Utilities|FlowControl|Delay 0.5)
  (Default|CollectItem (Variables|/Game/Blueprint/Player/BP_FirstPersonCharacter.BP_FirstPersonCharacter_C|GetBP_AC_Inventory _asbp_first_person_character) (Variables|Default|GetItem))
  (Utilities|IsValid _dialoguewhencollecting
    (:Is%20Valid
      (Default|StartNewDialogue (Variables|/Game/Blueprint/Player/BP_FirstPersonCharacter.BP_FirstPersonCharacter_C|GetHUD%20UI _asbp_first_person_character) _dialoguewhencollecting))
    (:Is%20Not%20Valid
      _))
  (Actor|DestroyActor))

(fn ConstructionScript
  (Components|StaticMesh|SetStaticMesh (Variables|Default|GetStaticMesh) "/Game/Developers/alexandrecoppens/PhotoFrame.PhotoFrame"))