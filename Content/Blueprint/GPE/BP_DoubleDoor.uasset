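; BP_DoubleDoor is an interactable double door built from two child actor doors, left and right church door leaves.
; It forwards Interacted, ShowWidget and HideWidget interface events to both child doors, so they respond together.
; Its own GetPrompt returns an empty string, and it holds no other logic of its own.
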(event EventBeginPlay)

(event Collision|EventActorBeginOverlap
  (params (OtherActor :type Actor%20Object%20Reference)))

(event EventTick
  (params (DeltaSeconds :type Float%20%28single-precision%29)))

(event EventInteracted
  (Class|BPIInteraction|Interacted(Message) (Variables|/Script/Engine.ChildActorComponent|GetChildActor (Variables|Default|GetBP_DoorChild_ChurchL)))
  (Class|BPIInteraction|Interacted(Message) (Variables|/Script/Engine.ChildActorComponent|GetChildActor (Variables|Default|GetBP_DoorChild_ChurchR))))

(event EventShowWidget
  (Class|BPIInteraction|ShowWidget(Message) (Variables|/Script/Engine.ChildActorComponent|GetChildActor (Variables|Default|GetBP_DoorChild_ChurchL)))
  (Class|BPIInteraction|ShowWidget(Message) (Variables|/Script/Engine.ChildActorComponent|GetChildActor (Variables|Default|GetBP_DoorChild_ChurchR))))

(event EventHideWidget
  (Class|BPIInteraction|HideWidget(Message) (Variables|/Script/Engine.ChildActorComponent|GetChildActor (Variables|Default|GetBP_DoorChild_ChurchL)))
  (Class|BPIInteraction|HideWidget(Message) (Variables|/Script/Engine.ChildActorComponent|GetChildActor (Variables|Default|GetBP_DoorChild_ChurchR))))

(fn ConstructionScript)

(fn GetPrompt
  (return ""))