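; BP_ItemToCollect is a world pickup that adds its Item to the player's inventory when interacted with.
; The construction script sets the static mesh and scale from the Item's mesh and ItemScale.
; Show and hide widget events toggle an outline overlay material on the mesh.
; Interacting calls CollectItem on the player's inventory component, starts an optional dialogue through the HUD, then destroys the actor.
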(event EventHideWidget
  (Rendering|Material|SetOverlayMaterial (Variables|Default|GetStaticMesh) 0 :!class /Script/Engine.MeshComponent))

(event EventShowWidget
  (Rendering|Material|SetOverlayMaterial (Variables|Default|GetStaticMesh) "/Game/Blueprint/GPE/M_Outline.M_Outline" :!class /Script/Engine.MeshComponent))

(event EventInteracted
  (bind _returnvalue (Game|GetPlayerCharacter 0))
  (bind _dialoguewhencollecting (Variables|Default|GetDialogueWhenCollecting))
  (bind _asbp_first_person_character (Utilities|Casting|CastToBP_FirstPersonCharacter _returnvalue))
  (Default|CollectItem (Variables|/Game/Blueprint/Player/BP_FirstPersonCharacter.BP_FirstPersonCharacter_C|GetBP_AC_Inventory _asbp_first_person_character) (Variables|Default|GetItem))
  (Utilities|IsValid _dialoguewhencollecting
    (:Is%20Valid
      (Default|StartNewDialogue (Variables|/Game/Blueprint/Player/BP_FirstPersonCharacter.BP_FirstPersonCharacter_C|GetHUD%20UI _asbp_first_person_character) _dialoguewhencollecting))
    (:Is%20Not%20Valid
      _))
  (Actor|DestroyActor))

(fn ConstructionScript
  (bind _item (Variables|Default|GetItem))
  (bind _staticmesh (Variables|Default|GetStaticMesh))
  (Utilities|IsValid _item
    (:Is%20Valid
      (Components|StaticMesh|SetStaticMesh _staticmesh (Variables|/Game/Blueprint/Inventory/BP_DA_Item.BP_DA_Item_C|GetMesh _item))
      (Transformation|SetRelativeScale3D _staticmesh (Variables|Default|GetItemScale)))))