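; Ambience manager actor that crossfades between outdoor and indoor 2D ambient sounds as the player enters and leaves its overlap area.
; BeginPlay starts the outdoor loop; player overlap spawns and fades in indoor ambience while fading out whichever outdoor instance is valid.
; Ending overlap spawns a fresh outdoor sound and fades out the indoor one, so each transition creates new audio components rather than reusing them.
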(event EventTick
  (params (DeltaSeconds :type Float%20%28single-precision%29)))

(event EventBeginPlay
  (bind _returnvalue (Audio|SpawnSound2D "/Game/05_SFX/SoundWaves/SW_Ambience_Outdoor.SW_Ambience_Outdoor" 1.0 1.0 0.0 0)))

(event Collision|EventActorBeginOverlap
  (params (OtherActor :type Actor%20Object%20Reference))
  (if (== OtherActor (Game|GetPlayerCharacter 0))
    (bind _returnvalue (Audio|SpawnSound2D "/Game/05_SFX/SoundWaves/SW_Ambience_Indoor.SW_Ambience_Indoor" 1.0 1.0 0.0 0))
    (Audio|Components|Audio|FadeIn _returnvalue 2.0 1.0 0.0 "Linear" :!class /Script/Engine.AudioComponent)
    (Utilities|IsValid (stale EventBeginPlay _returnvalue)
      (:Is%20Valid
        (Audio|Components|Audio|FadeOut (stale EventBeginPlay _returnvalue) 2.0 0.0 "Linear" :!class /Script/Engine.AudioComponent))
      (:Is%20Not%20Valid
        (Utilities|IsValid (stale Collision|EventActorEndOverlap _returnvalue)
          (:Is%20Valid
            (Audio|Components|Audio|FadeOut (stale Collision|EventActorEndOverlap _returnvalue) 2.0 0.0 "Linear" :!class /Script/Engine.AudioComponent)))))))

(event Collision|EventActorEndOverlap
  (params (OtherActor :type Actor%20Object%20Reference))
  (if (== OtherActor (Game|GetPlayerCharacter 0))
    (bind _returnvalue (Audio|SpawnSound2D "/Game/05_SFX/SoundWaves/SW_Ambience_Outdoor.SW_Ambience_Outdoor" 1.0 1.0 0.0 0))
    (Audio|Components|Audio|FadeIn _returnvalue 2.0 1.0 0.0 "Linear" :!class /Script/Engine.AudioComponent)
    (Utilities|IsValid (stale Collision|EventActorBeginOverlap _returnvalue)
      (:Is%20Valid
        (Audio|Components|Audio|FadeOut (stale Collision|EventActorBeginOverlap _returnvalue) 2.0 0.0 "Linear" :!class /Script/Engine.AudioComponent)))))

(fn ConstructionScript)